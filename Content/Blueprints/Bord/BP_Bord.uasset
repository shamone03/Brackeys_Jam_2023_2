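; BP_Bord is a player-controlled bird-like or board pawn ("Bord") with jump and sideways movement through Enhanced Input.
; BeginPlay adds the IMC_BordInput mapping context for its player controller.
; Jump applies a one-off upward physics force to SphereCollision, while Move feeds its X axis into movement input along the control rotation's right vector.
; Both input handlers print debug strings.
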(event Input|EnhancedActionEvents|EnhancedInputActionIA_Jump
  (params (ActionValue :type Boolean) (ElapsedSeconds :type Float%20%28double-precision%29) (TriggeredSeconds :type Float%20%28double-precision%29) (InputAction :type Input%20Action%20Object%20Reference :default "/Game/Blueprints/Input/IA_Jump.IA_Jump"))
  (:Started
    (Development|PrintString "Jumping")
    (Physics|AddForce (Variables|Default|GetSphereCollision) "0.000000,0.000000,50000.000000" "None" false)))

(event Input|EnhancedActionEvents|EnhancedInputActionIA_Move
  (params (ActionValue :type Float%20%28double-precision%29) (ElapsedSeconds :type Float%20%28double-precision%29) (TriggeredSeconds :type Float%20%28double-precision%29) (InputAction :type Input%20Action%20Object%20Reference :default "/Game/Blueprints/Input/IA_Move.IA_Move"))
  (bind _returnvalue (Pawn|GetControlRotation :!class /Script/Engine.Pawn))
  (:Triggered
    (Development|PrintString (Utilities|String|ToString(Float) (.x ActionValue)))
    (Pawn|Input|AddMovementInput (Math|Vector|GetRightVector (Math|Rotator|MakeRotator (.roll _returnvalue) 0.0 (.yaw _returnvalue))) (.x ActionValue) false)))

(event EventBeginPlay
  (bind _asplayer_controller (Utilities|Casting|CastToPlayerController (Pawn|GetController)))
  (Input|AddMappingContext (PlayerController|LocalPlayerSubsystems|GetEnhancedInputLocalPlayerSubsystem _asplayer_controller) "/Game/Blueprints/Input/IMC_BordInput.IMC_BordInput" 0 "(bIgnoreAllPressedKeysUntilRelease=True,bForceImmediately=False)"))

(event Collision|EventActorBeginOverlap
  (params (OtherActor :type Actor%20Object%20Reference)))

(event EventTick
  (params (DeltaSeconds :type Float%20%28single-precision%29)))

(fn ConstructionScript)