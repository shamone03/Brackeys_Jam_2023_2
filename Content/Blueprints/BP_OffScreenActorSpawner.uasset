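; BP_OffScreenActorSpawner periodically spawns actors just off screen in a side-view layout on the XZ plane.
; BeginPlay starts a looping timer that spawns ActorToSpawn every TimeBetweenSpawns.
; Each spawn picks a random left or right side, offsets X from the spawner by a random distance between ScreenRadius and ScreenRadius plus SpawnWidth, and picks a random height between MinHeight and MaxHeight, with Y fixed at zero.
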(event Custom|SpawnActor
  (bind _screenradius (Variables|Default|GetScreenRadius))
  (Game|SpawnActorfromClass (Variables|Default|GetActorToSpawn) (Math|Transform|MakeTransform (Math|Vector|MakeVector (+ (.X (Class|KismetMathLibrary|BreakVector3f (Transformation|GetActorLocation))) (* (- (* (Math|Random|RandomInteger 2) 2) 1) (Math|Random|RandomFloatinRange _screenradius (+ _screenradius (Variables|Default|GetSpawnWidth))))) 0.0 (Math|Random|RandomFloatinRange (Variables|Default|GetMinHeight) (Variables|Default|GetMaxHeight)))) "Undefined" "MultiplyWithRoot" 0 0))

(event EventBeginPlay
  (Utilities|Time|SetTimerbyEvent (delegate Custom|SpawnActor) (Variables|Default|GetTimeBetweenSpawns) true))

(event Collision|EventActorBeginOverlap
  (params (OtherActor :type Actor%20Object%20Reference)))

(event EventTick
  (params (DeltaSeconds :type Float%20%28single-precision%29)))

(fn ConstructionScript)