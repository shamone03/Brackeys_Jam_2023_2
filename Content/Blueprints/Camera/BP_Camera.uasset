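; BP_Camera is a camera actor that becomes the player's view target and follows the bird pawn along the X axis.
; On BeginPlay it pitches the spring arm and camera by opposite AimAngle values.
; Every tick it matches the pawn's X, then uses trigonometry on the vertical gap between a Cube reference and an offset pawn height to set arm length, clamped between close and far distances.
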(event EventBeginPlay
  (bind _returnvalue (Transformation|GetActorLocation))
  (bind _returnvalue_2 (Game|Player|GetPlayerPawn 0))
  (bind _cube (Variables|Default|GetCube))
  (bind _aimangle (Variables|Default|GetAimAngle))
  (bind _springarm (Variables|Default|GetSpringArm))
  (bind _camera (Variables|Actor|GetCamera))
  (bind _returnvalue_3 (Math|Float|Absolute(Float) _aimangle))
  (bind _returnvalue_4 (Transformation|GetWorldLocation _cube))
  (bind _returnvalue_5 (Transformation|GetActorLocation _returnvalue_2))
  (bind (_x _y _z) (Math|Vector|BreakVector _returnvalue))
  (bind _relativerotation (Variables|/Script/Engine.SceneComponent|GetRelativeRotation _camera))
  (bind _relativerotation_2 (Variables|/Script/Engine.SceneComponent|GetRelativeRotation _springarm))
  (bind _z_2 (Math|Vector|BreakVector _returnvalue_5))
  (bind _z_3 (Math|Vector|BreakVector _returnvalue_4))
  (bind (_roll _pitch _yaw) (Math|Rotator|BreakRotator _relativerotation))
  (bind (_roll_2 _pitch_2 _yaw_2) (Math|Rotator|BreakRotator _relativerotation_2))
  (bind _returnvalue_6 (- 9e+01 _returnvalue_3))
  (bind _returnvalue_7 (Math|Trig|Cos(Degrees) _returnvalue_6))
  (bind _returnvalue_8 (+ _z_2 1e+03))
  (bind _returnvalue_9 (- _z_3 _returnvalue_8))
  (bind _returnvalue_10 (Math|Float|Absolute(Float) _returnvalue_9))
  (bind _returnvalue_11 (/ _returnvalue_10 2.0))
  (bind _returnvalue_12 (/ _returnvalue_11 _returnvalue_7))
  (Game|Player|SetViewTargetwithBlend (Game|GetPlayerController (Variables|/Script/Engine.Pawn|GetPlayerState (Game|Player|GetPlayerPawn 0))) self 0.0 "VTBlend_Linear" 0.0 false)
  ;[1 1 1] angle the camera and spring arm
  (Transformation|SetRelativeRotation (Variables|Default|GetSpringArm) (Math|Rotator|MakeRotator _roll_2 (* (Variables|Default|GetAimAngle) -1.0) _yaw_2) false false)
  (Transformation|SetRelativeRotation (Variables|Actor|GetCamera) (Math|Rotator|MakeRotator _roll (Variables|Default|GetAimAngle) _yaw) false false)
  ;[1 1 1] update camera x position  to follow bird
  (Transformation|SetActorLocation (Math|Vector|MakeVector (.X (Math|Vector|BreakVector (Transformation|GetActorLocation (Game|Player|GetPlayerPawn 0)))) _y _z) false false)
  ;[1 1 1] adjust spring arm length (with restrictions)
  (if (>= _returnvalue_12 (Variables|Default|GetCloseCameraDistance))
    (if (<= _returnvalue_12 (Variables|Default|GetFarCameraDistance))
      (Variables|/Script/Engine.SpringArmComponent|SetTargetArmLength (Variables|Default|GetSpringArm) _returnvalue_12)
      (else
        (Variables|/Script/Engine.SpringArmComponent|SetTargetArmLength (Variables|Default|GetSpringArm) (Variables|Default|GetFarCameraDistance))))
    (else
      (Variables|/Script/Engine.SpringArmComponent|SetTargetArmLength (Variables|Default|GetSpringArm) (Variables|Default|GetCloseCameraDistance)))))

(event EventTick
  (params (DeltaSeconds :type Float%20%28single-precision%29))
  (bind _returnvalue (Transformation|GetActorLocation))
  (bind _returnvalue_2 (Game|Player|GetPlayerPawn 0))
  (bind _cube (Variables|Default|GetCube))
  (bind _aimangle (Variables|Default|GetAimAngle))
  (bind _returnvalue_3 (Math|Float|Absolute(Float) _aimangle))
  (bind _returnvalue_4 (Transformation|GetWorldLocation _cube))
  (bind _returnvalue_5 (Transformation|GetActorLocation _returnvalue_2))
  (bind (_x _y _z) (Math|Vector|BreakVector _returnvalue))
  (bind _z_2 (Math|Vector|BreakVector _returnvalue_5))
  (bind _z_3 (Math|Vector|BreakVector _returnvalue_4))
  (bind _returnvalue_6 (- 9e+01 _returnvalue_3))
  (bind _returnvalue_7 (Math|Trig|Cos(Degrees) _returnvalue_6))
  (bind _returnvalue_8 (+ _z_2 1e+03))
  (bind _returnvalue_9 (- _z_3 _returnvalue_8))
  (bind _returnvalue_10 (Math|Float|Absolute(Float) _returnvalue_9))
  (bind _returnvalue_11 (/ _returnvalue_10 2.0))
  (bind _returnvalue_12 (/ _returnvalue_11 _returnvalue_7))
  ;[1 1 1] update camera x position  to follow bird
  (Transformation|SetActorLocation (Math|Vector|MakeVector (.X (Math|Vector|BreakVector (Transformation|GetActorLocation (Game|Player|GetPlayerPawn 0)))) _y _z) false false)
  ;[1 1 1] adjust spring arm length (with restrictions)
  (if (>= _returnvalue_12 (Variables|Default|GetCloseCameraDistance))
    (if (<= _returnvalue_12 (Variables|Default|GetFarCameraDistance))
      (Variables|/Script/Engine.SpringArmComponent|SetTargetArmLength (Variables|Default|GetSpringArm) _returnvalue_12)
      (else
        (Variables|/Script/Engine.SpringArmComponent|SetTargetArmLength (Variables|Default|GetSpringArm) (Variables|Default|GetFarCameraDistance))))
    (else
      (Variables|/Script/Engine.SpringArmComponent|SetTargetArmLength (Variables|Default|GetSpringArm) (Variables|Default|GetCloseCameraDistance)))))

(fn ConstructionScript)