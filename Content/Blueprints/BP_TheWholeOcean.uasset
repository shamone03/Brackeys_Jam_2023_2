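; Ocean volume actor that gives BP_Bord actors buoyancy and audio feedback as they dive in and out.
; Begin and end overlap each cast to BP_Bord, then spawn and play an audio component and print a debug string.
; Every tick it scans components overlapping WaterCube and adds a delta-time-scaled upward force to the SphereCollision of each owning BP_Bord, once per overlapping component.
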(event EventBeginPlay)

(event Collision|EventActorBeginOverlap
  (params (OtherActor :type Actor%20Object%20Reference))
  (bind _asbp_bord (Utilities|Casting|CastToBP_Bord OtherActor))
  (Utilities|IsValid _asbp_bord
    (:Is%20Valid
      (bind _returnvalue (AddComponent|AddAudioComponent false))
      (Audio|Components|Audio|Play _returnvalue 0.0)
      (Development|PrintString "dive in"))))

(event EventTick
  (params (DeltaSeconds :type Float%20%28single-precision%29))
  (for _array_element (Class|PrimitiveComponent|GetOverlappingComponents (Variables|Default|GetWaterCube))
    (bind _asbp_bord (Utilities|Casting|CastToBP_Bord (Components|GetOwner _array_element)))
    (Utilities|IsValid _asbp_bord
      (:Is%20Valid
        (Physics|AddForce (Variables|/Game/Blueprints/Bord/BP_Bord.BP_Bord_C|GetSphereCollision _asbp_bord) (Math|Vector|MakeVector 0.0 0.0 (* DeltaSeconds 3.5e+05)) "None" false))
      (:Is%20Not%20Valid
        (Development|PrintString "not bord")))))

(event Collision|EventActorEndOverlap
  (params (OtherActor :type Actor%20Object%20Reference))
  (bind _asbp_bord (Utilities|Casting|CastToBP_Bord OtherActor))
  (Utilities|IsValid _asbp_bord
    (:Is%20Valid
      (bind _returnvalue (AddComponent|AddAudioComponent false))
      (Audio|Components|Audio|Play _returnvalue 0.0)
      (Development|PrintString "dive out"))))

(fn ConstructionScript)